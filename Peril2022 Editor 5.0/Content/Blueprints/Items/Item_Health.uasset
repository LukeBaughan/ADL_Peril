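; Health pickup item that heals the player who picks it up and then destroys itself.
; On BeginPlay it reuses the HUD's ammo label and value fields to show "Heals:" and the heal amount.
; The pickup action only works below max health, sending the heal through the damage interface message with a separate type and shield bypass.
; A brief, faint green camera fade gives feedback.
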(event EventBeginPlay
  (bind _myhud (Variables|Default|GetMyHud))
  (|CallParentFunction)
  (Rendering|Components|TextRender|SetText (Variables|/Game/CoreFiles/UI/WorldItemUI.WorldItemUI_C|GetAmmoText _myhud) "Heals:")
  (Rendering|Components|TextRender|SetText (Variables|/Game/CoreFiles/UI/WorldItemUI.WorldItemUI_C|GetAmmoValue _myhud) (Utilities|Text|ToText(Float) (Variables|Default|GetHealAmount) "HalfToEven")))

(event Collision|EventActorBeginOverlap
  (params (OtherActor :type Actor%20Object%20Reference)))

(event EventTick
  (params (DeltaSeconds :type Float%20%28single-precision%29))
  (|CallParentFunction DeltaSeconds) ; This node is disabled and will not be called.\nDrag off pins to build functionality.
)

(event EventPickUpAction
  (params (Player :type Player%20Character%20Object%20Reference))
  (if (< (Variables|/Game/Blueprints/Characters/PlayerCharacter.PlayerCharacter_C|GetHealth Player) (Variables|/Game/Blueprints/Characters/PlayerCharacter.PlayerCharacter_C|GetMaxHealth Player))
    (Class|DamageInterface|DamageInterface(Message) Player (Variables|Default|GetHealAmount) "0, 0, 0" 0.0 0 false "NewEnumerator1" "0, 0, 0" "0, 0, 0" true)
    (CameraFades|StartCameraFade (Game|GetPlayerCameraManager 0) 0.0 0.05 0.1 "(R=0.000000,G=1.000000,B=0.056106,A=1.000000)" false false)
    (Actor|DestroyActor)))

(fn ConstructionScript
  (|CallParentFunction))