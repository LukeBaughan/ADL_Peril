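; Colour-coded key pickup that hands itself to the player on pickup through PickUpKey, without running the parent pickup logic.
; The construction script tints the paper sprite to match the Colour enum (red, blue or green) and sets the point light to black in every case.
; BeginPlay builds the name from the colour, shows it on the HUD widget with a door-opening quote and hides the ammo fields.
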(event EventBeginPlay
  (bind _myhud (Variables|Default|GetMyHud))
  (|CallParentFunction)
  (bind _output_get (Variables|Default|SetName (Utilities|String|StringToName (Utilities|String|Append (Utilities|String|EnumtoString (Variables|Default|GetColour)) " " "Key"))))
  (Rendering|Components|TextRender|SetText (Variables|/Game/CoreFiles/UI/WorldItemUI.WorldItemUI_C|GetNameText _myhud) (Utilities|Text|ToText(Name) _output_get))
  (Widget|SetVisibility (Variables|/Game/CoreFiles/UI/WorldItemUI.WorldItemUI_C|GetAmmoValue _myhud) "Hidden")
  (Rendering|Components|TextRender|SetText (Variables|/Game/CoreFiles/UI/WorldItemUI.WorldItemUI_C|GetQuote _myhud) "Opens a door"))

(event EventPickUpAction
  (params (Player :type Player%20Character%20Object%20Reference))
  (Default|PickUpKey Player self))

(fn ConstructionScript
  (bind _papersprite (Variables|Default|GetPaperSprite))
  (bind _pointlight (Variables|Default|GetPointLight))
  (|CallParentFunction)
  (switch Utilities|FlowControl|Switch|SwitchonKeyColour (Variables|Default|GetColour)
    (:NewEnumerator0
      (Sprite|SetSpriteColor _papersprite "(R=1.000000,G=0.008162,B=0.000000,A=1.000000)")
      (Rendering|Components|Light|SetLightColor :self _pointlight))
    (:NewEnumerator1
      (Sprite|SetSpriteColor _papersprite "(R=0.000000,G=0.097714,B=1.000000,A=1.000000)")
      (Rendering|Components|Light|SetLightColor :self _pointlight))
    (:NewEnumerator2
      (Sprite|SetSpriteColor _papersprite "(R=0.067848,G=0.520833,B=0.045256,A=1.000000)")
      (Rendering|Components|Light|SetLightColor :self _pointlight))))