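; Slime floor cube is a level hazard that has the player character run an environmental damage check on entering or leaving its box.
; When projectile spawning is enabled, it waits a start delay, then spawns a Slimeball 400 units above itself immediately and on a looping timer.
; The construction script scales particle parameters with the mesh's X scale.
; Unconnected editor logic for toggling walls and a ceiling remains in the graph but never runs.
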(event OnComponentBeginOverlap(Box)
  (params (OverlappedComponent :type Primitive%20Component%20Object%20Reference) (OtherActor :type Actor%20Object%20Reference) (OtherComp :type Primitive%20Component%20Object%20Reference) (OtherBodyIndex :type Integer) (bFromSweep :type Boolean) (SweepResult :type Hit%20Result%20Structure%20%28by%20ref%29))
  (bind _asplayer_character (Utilities|Casting|CastToPlayerCharacter OtherActor))
  (Default|EnviroDamageCheck _asplayer_character))

(event OnComponentEndOverlap(Box)
  (params (OverlappedComponent :type Primitive%20Component%20Object%20Reference) (OtherActor :type Actor%20Object%20Reference) (OtherComp :type Primitive%20Component%20Object%20Reference) (OtherBodyIndex :type Integer))
  (bind _asplayer_character (Utilities|Casting|CastToPlayerCharacter OtherActor))
  (Default|EnviroDamageCheck _asplayer_character))

(event Custom|Start%20Spawn%20Timer
  (CallFunction|SpawnProjectile)
  (Utilities|Time|SetTimerbyEvent (delegate Custom|Spawn%20Projectile) (Variables|Default|GetSlimeProjectileRate) true))

(event Custom|Spawn%20Projectile
  (bind _returnvalue (Transformation|GetActorTransform))
  (Game|SpawnActorfromClass "/Game/CoreFiles/Characters/Enemy/Slimeball.Slimeball_C" (Math|Transform|MakeTransform (Math|Vector|MakeVector (.x (.location _returnvalue)) (.y (.location _returnvalue)) (+ (.z (.location _returnvalue)) 4e+02)) (.rotation _returnvalue) (.scale _returnvalue)) "Undefined" 0 0))

(event EventBeginPlay
  (if (Variables|Default|GetSpawn%20Projectile?)
    (Utilities|FlowControl|Delay (Variables|Default|GetProjectileStartDelay))
    (CallFunction|StartSpawnTimer)))

(fn ConstructionScript
  (bind _particlesystem (Variables|Default|GetParticleSystem))
  (bind _staticmesh_0 (Variables|Default|GetStaticMesh_0))
  (bind _returnvalue (Transformation|GetWorldScale _staticmesh_0))
  (bind _x (Math|Vector|BreakVector _returnvalue))
  (Effects|Components|ParticleSystem|SetFloatParameter _particlesystem "Bits" (* _x 1e+02))
  (Effects|Components|ParticleSystem|SetFloatParameter _particlesystem "RateScale" _x))