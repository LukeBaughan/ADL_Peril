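; Level trigger volume that spawns a set of enemies at linked spawn points the first time the player overlaps its box.
; Tinted teleport particles play at each point, then after a delay each is replaced by the enemy class at the matching array index.
; If set to spawn aggressive, each enemy is handed the triggering player as its target.
; A separate event draws debug traces to the linked spawn points.
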(event OnComponentBeginOverlap(Box)
  (params (OverlappedComponent :type Primitive%20Component%20Object%20Reference) (OtherActor :type Actor%20Object%20Reference) (OtherComp :type Primitive%20Component%20Object%20Reference) (OtherBodyIndex :type Integer) (bFromSweep :type Boolean) (SweepResult :type Hit%20Result%20Structure%20%28by%20ref%29))
  ;[1 1 1] On Overlap spawn enemies
  (bind _asplayer_character (Utilities|Casting|CastToPlayerCharacter OtherActor))
  (Utilities|FlowControl|DoOnce false
    (:Completed
      (Variables|Default|SetMyTarget _asplayer_character)
      (CallFunction|SpawnEmitter))))

(event Custom|Spawn%20Enemies
  ;[1 1 1] Spawn Enemies
  (for (_array_element _array_index) (Variables|Default|GetMyTeleportParticle)
    (bind _returnvalue (Game|SpawnActorfromClass (Utilities|Array|Get(acopy) (Variables|Default|GetMyEnemies) _array_index) (Math|Transform|MakeTransform (Transformation|GetWorldLocation _array_element) (Transformation|GetWorldRotation _array_element) "1,1,1") "AdjustIfPossibleButAlwaysSpawn" 0 false 0))
    (Components|DestroyComponent _array_element)
    (if (Variables|Default|GetSpawn%20Aggressive?)
      (Default|Perception(Manual) _returnvalue (Variables|Default|GetMyTarget))))
  (Utilities|Array|Clear (Variables|Default|GetMyTeleportParticle)))

(event Custom|Show%20My%20Spawn%20Points
  ;[1 1 1] Show Connected ACtors
  (Utilities|FlowControl|Sequence
    (:then_0
      (for _array_element (Variables|Default|GetMySpawnPoints)
        (Collision|LineTraceByChannel (Transformation|GetWorldLocation (Variables|Default|GetBillboard)) (Transformation|GetWorldLocation (Variables|/Game/Blueprints/LevelCreation/SpawnPoint.SpawnPoint_C|GetBillboard _array_element)) "TraceTypeQuery1" false 0 "Persistent" true "(R=1.000000,G=0.000000,B=0.000000,A=1.000000)" "(R=0.000000,G=1.000000,B=0.000000,A=1.000000)" 3e+01)))))

(event Custom|Spawn%20Emitter
  (bind _teleportcolour (Variables|Default|GetTeleportColour))
  ;[1 1 1] Spawn Teleport Particles
  (for _array_element (Variables|Default|GetMySpawnPoints)
    (bind _returnvalue (Effects|SpawnEmitteratLocation "/Game/CoreFiles/Graphics/TeleportParticle.TeleportParticle" (Transformation|GetWorldLocation (Variables|/Game/Blueprints/LevelCreation/SpawnPoint.SpawnPoint_C|GetBillboard _array_element)) (Transformation|GetActorRotation _array_element) "2.000000,2.000000,2.000000"))
    (Utilities|Array|Add (Variables|Default|GetMyTeleportParticle) _returnvalue)
    (Effects|Components|ParticleSystem|SetVectorParameter _returnvalue "TeleportColour" (Math|Vector|MakeVector (.r _teleportcolour) (.g _teleportcolour) (.b _teleportcolour))))
  (Utilities|FlowControl|Delay (Variables|Default|GetSpawnDelay))
  (CallFunction|SpawnEnemies))

(fn ConstructionScript)