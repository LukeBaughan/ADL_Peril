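; Wall switch that players use to trigger linked level actors such as doors, optionally gated by a key card.
; Interact checks the player's KeyInv for RequiredKey, shows HUD notifications, and has a SingleUse option built on DoOnce.
; Activate sends TriggerResponseMessage to every actor in MyTargets.
; ShowMyDoors draws debug line traces to each target for editor visualization and prints a warning for unconnected ones.
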(event Custom|Activate
  ;[1 1 1] Trigger linked Actors
  (for _array_element (Variables|Default|GetMyTargets)
    (Class|TriggerResponse|TriggerResponse(Message) _array_element)))

(event Custom|Show%20My%20Doors
  ;[1 1 1] Show my Targets in Editor
  (Utilities|FlowControl|Sequence
    (:then_0
      (for _array_element (Variables|Default|GetMyTargets)
        (Utilities|IsValid _array_element
          (:Is%20Valid
            (Collision|LineTraceByChannel (Transformation|GetWorldLocation (Variables|Default|GetBox)) (Transformation|GetActorLocation _array_element) "TraceTypeQuery1" false 0 "ForDuration"))
          (:Is%20Not%20Valid
            (Development|PrintString "Door not connected!!")))))))

(event EventInteract
  (params (Player :type Player%20Character%20Object%20Reference))
  (bind _keyinv (Variables|/Game/Blueprints/Characters/PlayerCharacter.PlayerCharacter_C|GetKeyInv Player))
  (bind _requiredkey (Variables|Default|GetRequiredKey))
  (bind _myhud (Variables|/Game/Blueprints/Characters/PlayerCharacter.PlayerCharacter_C|GetMyHud Player))
  ;[1 1 1] On Used
  (if (not (Utilities|Enum|Equal(Enum) (Variables|Default|GetRequiredKey) "NewEnumerator3"))
    (if (Utilities|Array|IsValidIndex _keyinv (Utilities|Array|FindItem _keyinv _requiredkey))
      (if (Variables|Default|GetSingleUse)
        (Utilities|FlowControl|DoOnce false
          (:Completed
            _)))
      (CallFunction|Activate)
      (Utilities|FlowControl|DoOnce false
        (:Completed
          (Default|DisplayNotification _myhud "Door Unlocked." false)))
      (else
        (Default|DisplayNotification _myhud (Utilities|String|Append (Utilities|String|EnumtoString _requiredkey) " " "Key Card Required.") false)))
    (else
      (if (Variables|Default|GetSingleUse)
        (Utilities|FlowControl|DoOnce false
          (:Completed
            _)))
      (CallFunction|Activate)
      (Default|DisplayNotification _myhud "Switch Used" false))))

(fn ConstructionScript)