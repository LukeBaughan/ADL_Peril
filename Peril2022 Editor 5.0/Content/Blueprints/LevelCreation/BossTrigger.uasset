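; Boss encounter trigger that seals the arena and spawns a boss when the player enters.
; Box overlap fires once, shaking the camera, notifying the HUD, locking MyDoors and playing a teleport effect before a timed spawn at BossSpawnPoint.
; Boss destruction opens the doors and removes the trigger, or rearms it if the player died; Reset also cancels the timer.
; A helper event draws debug traces to linked doors and spawn point.
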(event OnComponentBeginOverlap(Box)
  (params (OverlappedComponent :type Primitive%20Component%20Object%20Reference) (OtherActor :type Actor%20Object%20Reference) (OtherComp :type Primitive%20Component%20Object%20Reference) (OtherBodyIndex :type Integer) (bFromSweep :type Boolean) (SweepResult :type Hit%20Result%20Structure%20%28by%20ref%29))
  ;[1 1 1] On Overlap Close All Doors
  (bind _asplayer_character (Utilities|Casting|CastToPlayerCharacter OtherActor))
  (Utilities|FlowControl|DoOnce false
    (:Completed
      (Class|PlayerCameraManager|PlayCameraShake (Game|GetPlayerCameraManager 0) "/Game/CoreFiles/Characters/LongCameraShake.LongCameraShake_C" 1.0 "CameraLocal" "0, 0, 0")
      (Default|DisplayNotification (Variables|/Game/Blueprints/Characters/PlayerCharacter.PlayerCharacter_C|GetMyHud _asplayer_character) "A powerful enemy approaches!" false)
      (Variables|Default|SetMyTarget _asplayer_character)
      (for _array_element (Variables|Default|GetMyDoors)
        (if (Variables|/Game/Blueprints/LevelCreation/Door.Door_C|GetOpen? _array_element)
          (Default|DoorClose _array_element))
        (Variables|/Game/Blueprints/LevelCreation/Door.Door_C|SetRequired _array_element "NewEnumerator6")
        (Default|UpdateLightColour _array_element))
      (CallFunction|SpawnEmitter)
      (bind _returnvalue (Utilities|Time|SetTimerbyEvent (delegate Custom|Spawn%20Boss) 3.0))
      (Variables|Default|SetBoss%20Spawn%20Timer _returnvalue))))

(event Custom|Spawn%20Boss
  ;[1 1 1] Spawn Boss
  (Components|DestroyComponent (Variables|Default|GetMyTeleportParticle))
  (Variables|Default|SetMyTeleportParticle 0)
  (bind _returnvalue (Game|SpawnActorfromClass (Variables|Default|GetBoss) (Transformation|GetActorTransform (Variables|Default|GetBossSpawnPoint)) "AdjustIfPossibleButAlwaysSpawn" 0 false 0))
  (Default|Perception(Manual) _returnvalue (Variables|Default|GetMyTarget))
  (Game|BindEventtoOnDestroyed _returnvalue (delegate Custom|Boss%20Defeated))
  (Variables|/Game/CoreFiles/Characters/Enemy/Enemy.Enemy_C|SetActivated _returnvalue true))

(event Custom|Reset%20Trigger
  ;[1 1 1] On Overlap Close All Doors
  (Utilities|FlowControl|DoOnce false) ; enters at Reset
)

(event Custom|Boss%20Defeated
  (params (DestroyedActor :type Actor%20Object%20Reference))
  (bind _mydoors (Variables|Default|GetMyDoors))
  ;[1 1 1] Boss Defeated
  (bind _asplayer_character (Utilities|Casting|CastToPlayerCharacter (Variables|Default|GetMyTarget)))
  (if (Variables|/Game/Blueprints/Characters/PlayerCharacter.PlayerCharacter_C|GetDead _asplayer_character)
    (for _array_element _mydoors
      (Variables|/Game/Blueprints/LevelCreation/Door.Door_C|SetRequired _array_element (Variables|/Game/Blueprints/LevelCreation/Door.Door_C|GetDefaultRequired _array_element))
      (Default|UpdateLightColour _array_element))
    (CallFunction|ResetTrigger)
    (Utilities|IsValid (Variables|Default|GetMyTeleportParticle)
      (:Is%20Valid
        (Components|DestroyComponent (Variables|Default|GetMyTeleportParticle))
        (Variables|Default|SetMyTeleportParticle 0)))
    (else
      (for _array_element_2 _mydoors
        (Variables|/Game/Blueprints/LevelCreation/Door.Door_C|SetRequired _array_element_2 "NewEnumerator0")
        (Default|UpdateLightColour _array_element_2)
        (if (not (Variables|/Game/Blueprints/LevelCreation/Door.Door_C|GetOpen? _array_element_2))
          (Default|DoorOpen _array_element_2)))
      (Actor|DestroyActor))))

(event Custom|Reset
  (Utilities|Time|ClearandInvalidateTimerbyHandle (Variables|Default|GetBoss%20Spawn%20Timer))
  (for _array_element (Variables|Default|GetMyDoors)
    (Variables|/Game/Blueprints/LevelCreation/Door.Door_C|SetRequired _array_element (Variables|/Game/Blueprints/LevelCreation/Door.Door_C|GetDefaultRequired _array_element))
    (Default|UpdateLightColour _array_element))
  (CallFunction|ResetTrigger)
  (Utilities|IsValid (Variables|Default|GetMyTeleportParticle)
    (:Is%20Valid
      (Components|DestroyComponent (Variables|Default|GetMyTeleportParticle))
      (Variables|Default|SetMyTeleportParticle 0))))

(event Custom|Show%20My%20Doors%20and%20Spawn
  (bind _bossspawnpoint (Variables|Default|GetBossSpawnPoint))
  (bind _billboard (Variables|Default|GetBillboard))
  (bind _returnvalue (Transformation|GetWorldLocation _billboard))
  ;[1 1 1] Show Connected ACtors
  (Utilities|FlowControl|Sequence
    (:then_0
      (for _array_element (Variables|Default|GetMyDoors)
        (Collision|LineTraceByChannel _returnvalue (Transformation|GetActorLocation _array_element) "TraceTypeQuery1" false 0 "ForDuration")))
    (:then_1
      (Utilities|IsValid _bossspawnpoint
        (:Is%20Valid
          (Collision|LineTraceByChannel _returnvalue (Transformation|GetWorldLocation (Variables|/Game/Blueprints/LevelCreation/SpawnPoint.SpawnPoint_C|GetBillboard _bossspawnpoint)) "TraceTypeQuery1" false 0 "ForDuration"))))))

(event Custom|Spawn%20Emitter
  (bind _teleportcolour (Variables|Default|GetTeleportColour))
  (bind _returnvalue (Effects|SpawnEmitteratLocation "/Game/CoreFiles/Graphics/TeleportParticle.TeleportParticle" (Transformation|GetActorLocation (Variables|Default|GetBossSpawnPoint)) "0, 0, 0" "8.000000,8.000000,8.000000"))
  (bind _output_get (Variables|Default|SetMyTeleportParticle _returnvalue))
  (Effects|Components|ParticleSystem|SetVectorParameter _output_get "TeleportColour" (Math|Vector|MakeVector (.r _teleportcolour) (.g _teleportcolour) (.b _teleportcolour))))

(fn ConstructionScript)