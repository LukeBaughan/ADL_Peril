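; LevelHelper is a per-level utility actor that validates level setup, manages generated geometry and stages a death-stats view.
; Checks report missing player, end switch or enemies through prints and a billboard sprite.
; BeginPlay rebuilds floor-cube and room-spawner walls (in ordered passes) and ceilings, then shows the level name on the HUD.
; StartStats switches to EndCamera, removes ceilings, occluders and corpses, and spawns flipbook StatActors above recorded enemy deaths.
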(event Custom|Start%20Stats
  (bind _end_camera (Variables|Default|GetEnd%20Camera))
  ;[1 1 1] Stats
  (Utilities|FlowControl|Sequence
    (:then_0
      (Utilities|IsValid _end_camera
        (:Is%20Valid
          (Game|Player|SetViewTargetwithBlend (Game|GetPlayerController 0) _end_camera 0.0 "VTBlend_Linear" 0.0 false))))
    (:then_1
      (CallFunction|TurnOffCeilings))
    (:then_2
      (bind _outactors (Actor|GetAllActorsOfClass "/Game/CoreFiles/WorldOccluderBox_Blueprint.WorldOccluderBox_Blueprint_C"))
      (for _array_element _outactors
        (Actor|DestroyActor _array_element)))
    (:then_3
      (CallFunction|SpawnStatActors)
      (bind _outactors_2 (Actor|GetAllActorsOfClass "/Script/Engine.ExponentialHeightFog")))
    (:then_4
      (bind _outactors_3 (Actor|GetAllActorsOfClass "/Game/CoreFiles/Characters/Corpse.Corpse_C"))
      (for _array_element_2 _outactors_3
        (Actor|DestroyActor _array_element_2)))))

(event Custom|Check%20For%20Issues
  (bind _textduration (Variables|Default|GetTextDuration))
  (bind _billboard (Variables|Default|GetBillboard))
  ;[1 1 1] Level Checks
  (Variables|Default|SetErrorCount 0)
  (Development|PrintString "====Start Check====" true true "(R=1.000000,G=0.000000,B=0.763262,A=1.000000)" (Variables|Default|GetTextDuration))
  (CallFunction|CheckforPlayer)
  (CallFunction|CheckforEndLevelSwitch)
  (CallFunction|CountEnemies)
  (if (> (Variables|Default|GetErrorCount) 0)
    (Development|PrintString (Utilities|String|Append "==" (Utilities|String|ToString(Integer) (Variables|Default|GetErrorCount)) " Errors Found!" "==") true true "(R=1.000000,G=0.045439,B=0.000000,A=1.000000)" _textduration)
    (Rendering|Components|Sprite|SetSprite _billboard "/Game/CoreFiles/Graphics/helpe2.helpe2")
    (else
      (Development|PrintString "==No Errors found!==" true true "(R=0.073642,G=1.000000,B=0.000000,A=1.000000)" _textduration)
      (Rendering|Components|Sprite|SetSprite _billboard "/Game/CoreFiles/Graphics/helper.helper"))))

(event Custom|Turn%20Off%20Ceilings
  ;[1 1 1] Toggle Ceiling
  (Utilities|FlowControl|Sequence
    (:then_0
      (bind _outactors (Actor|GetAllActorsOfClass "/Game/Blueprints/LevelCreation/EditorFloorCube.EditorFloorCube_C"))
      (for _array_element _outactors
        (Default|DestroyCeiling _array_element)))
    (:then_1
      (bind _outactors_2 (Actor|GetAllActorsOfClass "/Game/Blueprints/LevelCreation/SlimeFloorCube.SlimeFloorCube_C"))
      (for _array_element_2 _outactors_2
        (Default|DestroyCeiling _array_element_2)))
    (:then_2
      (bind _outactors_3 (Actor|GetAllActorsOfClass "/Game/Blueprints/LevelCreation/EditorRoomSpawner2.EditorRoomSpawner2_C"))
      (for _array_element_3 _outactors_3
        (Default|DestroyCeiling _array_element_3)))
    (:then_3
      (Variables|Default|SetCeiling%20On false))))

(event Custom|Turn%20Off%20Walls
  ;[1 1 1] Toggle Walls
  (Utilities|FlowControl|Sequence
    (:then_0
      (bind _outactors (Actor|GetAllActorsOfClass "/Game/Blueprints/LevelCreation/EditorFloorCube.EditorFloorCube_C"))
      (for _array_element _outactors
        (Default|DestroyWalls _array_element)))
    (:then_1
      (bind _outactors_2 (Actor|GetAllActorsOfClass "/Game/Blueprints/LevelCreation/SlimeFloorCube.SlimeFloorCube_C"))
      (for _array_element_2 _outactors_2
        (Default|DestroyWalls _array_element_2)))
    (:then_2
      (bind _outactors_3 (Actor|GetAllActorsOfClass "/Game/Blueprints/LevelCreation/EditorRoomSpawner2.EditorRoomSpawner2_C"))
      (for _array_element_3 _outactors_3
        (Default|DestroyWalls _array_element_3)))
    (:then_3
      (Variables|Default|SetWalls%20On false))))

(event Custom|Turn%20On%20Ceilings
  ;[1 1 1] Toggle Ceiling
  (Utilities|FlowControl|Sequence
    (:then_0
      (bind _outactors (Actor|GetAllActorsOfClass "/Game/Blueprints/LevelCreation/EditorFloorCube.EditorFloorCube_C"))
      (for _array_element _outactors
        (Default|CreateCeiling _array_element)))
    (:then_1
      (bind _outactors_2 (Actor|GetAllActorsOfClass "/Game/Blueprints/LevelCreation/SlimeFloorCube.SlimeFloorCube_C"))
      (for _array_element_2 _outactors_2
        (Default|CreateCeiling _array_element_2)))
    (:then_2
      (bind _outactors_3 (Actor|GetAllActorsOfClass "/Game/Blueprints/LevelCreation/EditorRoomSpawner2.EditorRoomSpawner2_C"))
      (for _array_element_3 _outactors_3
        (Default|CreateCeiling _array_element_3)))
    (:then_3
      (Variables|Default|SetCeiling%20On true))))

(event Custom|Turn%20On%20Walls
  ;[1 1 1] Toggle Walls
  (Utilities|FlowControl|Sequence
    (:then_0
      (bind _outactors (Actor|GetAllActorswithTag "RoomFloor"))
      (for _array_element _outactors
        (bind _aseditor_floor_cube (Utilities|Casting|CastToEditorFloorCube _array_element))
        (Default|CreateWalls _aseditor_floor_cube)))
    (:then_1
      (bind _outactors_2 (Actor|GetAllActorsOfClass "/Game/Blueprints/LevelCreation/EditorFloorCube.EditorFloorCube_C"))
      (for _array_element_2 _outactors_2
        (if (and (not (Actor|ActorHasTag _array_element_2 "RoomFloor")) (== (Variables|/Game/Blueprints/LevelCreation/EditorFloorCube.EditorFloorCube_C|GetRoomHeight _array_element_2) 2))
          (Default|CreateWalls _array_element_2))))
    (:then_2
      (bind _outactors_3 (Actor|GetAllActorsOfClass "/Game/Blueprints/LevelCreation/EditorFloorCube.EditorFloorCube_C"))
      (for _array_element_3 _outactors_3
        (if (and (not (Actor|ActorHasTag _array_element_3 "RoomFloor")) (== (Variables|/Game/Blueprints/LevelCreation/EditorFloorCube.EditorFloorCube_C|GetRoomHeight _array_element_3) 1))
          (Default|CreateWalls _array_element_3))))
    (:then_3
      (bind _outactors_4 (Actor|GetAllActorsOfClass "/Game/Blueprints/LevelCreation/SlimeFloorCube.SlimeFloorCube_C"))
      (for _array_element_4 _outactors_4
        (Default|CreateWalls _array_element_4)))
    (:then_4
      (bind _outactors_5 (Actor|GetAllActorsOfClass "/Game/Blueprints/LevelCreation/EditorRoomSpawner2.EditorRoomSpawner2_C"))
      (for _array_element_5 _outactors_5
        (Default|CreateWalls _array_element_5)))
    (:then_5
      (Variables|Default|SetWalls%20On true))))

(event Custom|Toggle%20Walls
  ;[1 1 1] Toggle Walls
  (if (Variables|Default|GetWalls%20On)
    (Utilities|FlowControl|Sequence
      (:then_0
        (bind _outactors (Actor|GetAllActorsOfClass "/Game/Blueprints/LevelCreation/EditorFloorCube.EditorFloorCube_C"))
        (for _array_element _outactors
          (Default|DestroyWalls _array_element)))
      (:then_1
        (bind _outactors_2 (Actor|GetAllActorsOfClass "/Game/Blueprints/LevelCreation/SlimeFloorCube.SlimeFloorCube_C"))
        (for _array_element_2 _outactors_2
          (Default|DestroyWalls _array_element_2)))
      (:then_2
        (bind _outactors_3 (Actor|GetAllActorsOfClass "/Game/Blueprints/LevelCreation/EditorRoomSpawner2.EditorRoomSpawner2_C"))
        (for _array_element_3 _outactors_3
          (Default|DestroyWalls _array_element_3)))
      (:then_3
        (Variables|Default|SetWalls%20On false)))
    (else
      (Utilities|FlowControl|Sequence
        (:then_0
          (bind _outactors_4 (Actor|GetAllActorswithTag "RoomFloor"))
          (for _array_element_4 _outactors_4
            (bind _aseditor_floor_cube (Utilities|Casting|CastToEditorFloorCube _array_element_4))
            (Default|CreateWalls _aseditor_floor_cube)))
        (:then_1
          (bind _outactors_5 (Actor|GetAllActorsOfClass "/Game/Blueprints/LevelCreation/EditorFloorCube.EditorFloorCube_C"))
          (for _array_element_5 _outactors_5
            (if (and (not (Actor|ActorHasTag _array_element_5 "RoomFloor")) (== (Variables|/Game/Blueprints/LevelCreation/EditorFloorCube.EditorFloorCube_C|GetRoomHeight _array_element_5) 2))
              (Default|CreateWalls _array_element_5))))
        (:then_2
          (bind _outactors_6 (Actor|GetAllActorsOfClass "/Game/Blueprints/LevelCreation/EditorFloorCube.EditorFloorCube_C"))
          (for _array_element_6 _outactors_6
            (if (and (not (Actor|ActorHasTag _array_element_6 "RoomFloor")) (== (Variables|/Game/Blueprints/LevelCreation/EditorFloorCube.EditorFloorCube_C|GetRoomHeight _array_element_6) 1))
              (Default|CreateWalls _array_element_6))))
        (:then_3
          (bind _outactors_7 (Actor|GetAllActorsOfClass "/Game/Blueprints/LevelCreation/SlimeFloorCube.SlimeFloorCube_C"))
          (for _array_element_7 _outactors_7
            (Default|CreateWalls _array_element_7)))
        (:then_4
          (bind _outactors_8 (Actor|GetAllActorsOfClass "/Game/Blueprints/LevelCreation/EditorRoomSpawner2.EditorRoomSpawner2_C"))
          (for _array_element_8 _outactors_8
            (Default|CreateWalls _array_element_8)))
        (:then_5
          (Variables|Default|SetWalls%20On true))))))

(event Custom|Toggle%20Ceilings
  ;[1 1 1] Toggle Ceiling
  (if (Variables|Default|GetCeiling%20On)
    (Utilities|FlowControl|Sequence
      (:then_0
        (bind _outactors (Actor|GetAllActorsOfClass "/Game/Blueprints/LevelCreation/EditorFloorCube.EditorFloorCube_C"))
        (for _array_element _outactors
          (Default|DestroyCeiling _array_element)))
      (:then_1
        (bind _outactors_2 (Actor|GetAllActorsOfClass "/Game/Blueprints/LevelCreation/SlimeFloorCube.SlimeFloorCube_C"))
        (for _array_element_2 _outactors_2
          (Default|DestroyCeiling _array_element_2)))
      (:then_2
        (bind _outactors_3 (Actor|GetAllActorsOfClass "/Game/Blueprints/LevelCreation/EditorRoomSpawner2.EditorRoomSpawner2_C"))
        (for _array_element_3 _outactors_3
          (Default|DestroyCeiling _array_element_3)))
      (:then_3
        (Variables|Default|SetCeiling%20On false)))
    (else
      (Utilities|FlowControl|Sequence
        (:then_0
          (bind _outactors_4 (Actor|GetAllActorsOfClass "/Game/Blueprints/LevelCreation/EditorFloorCube.EditorFloorCube_C"))
          (for _array_element_4 _outactors_4
            (Default|CreateCeiling _array_element_4)))
        (:then_1
          (bind _outactors_5 (Actor|GetAllActorsOfClass "/Game/Blueprints/LevelCreation/SlimeFloorCube.SlimeFloorCube_C"))
          (for _array_element_5 _outactors_5
            (Default|CreateCeiling _array_element_5)))
        (:then_2
          (bind _outactors_6 (Actor|GetAllActorsOfClass "/Game/Blueprints/LevelCreation/EditorRoomSpawner2.EditorRoomSpawner2_C"))
          (for _array_element_6 _outactors_6
            (Default|CreateCeiling _array_element_6)))
        (:then_3
          (Variables|Default|SetCeiling%20On true))))))

(event Custom|Spawn%20Stat%20Actors
  ;[1 1 1] Stats
  (for _array_element (Variables|Default|GetEnemyDeathList)
    (Game|SpawnActorfromClass "/Game/CoreFiles/UI/StatScreen/StatActor.StatActor_C" (Math|Transform|MakeTransform (Math|Vector|MakeVector (.X (Math|Vector|BreakVector (.Location (Utilities|Struct|BreakDeathStatStruct _array_element)))) (.Y (Math|Vector|BreakVector (.Location (Utilities|Struct|BreakDeathStatStruct _array_element)))) (+ 1e+03 (Math|Random|RandomFloat))) (Math|Rotator|MakeRotator 0.0 0.0 (.Yaw (Math|Rotator|BreakRotator (.DeathRotation (Utilities|Struct|BreakDeathStatStruct _array_element))))) (* (.CorpseFlipbookScale (Utilities|Struct|BreakDeathStatStruct _array_element)) 4.0)) "AlwaysSpawn" 0 0 (.DeathFlipbook (Utilities|Struct|BreakDeathStatStruct _array_element)) 0 0)))

(event Custom|Check%20For%20Player
  (bind _textduration (Variables|Default|GetTextDuration))
  ;[1 1 1] Level Checks
  (bind _outactors (Actor|GetAllActorsOfClass "/Game/Blueprints/Characters/PlayerCharacter.PlayerCharacter_C"))
  (if (Utilities|Array|IsValidIndex _outactors)
    (Development|PrintString (Utilities|String|Append (Utilities|String|ToString(Integer) (Utilities|Array|Length _outactors)) " Player found") true true "(R=0.072053,G=1.000000,B=0.000000,A=1.000000)" _textduration)
    (else
      (Development|PrintString "!WARNING! - No FirstPersonCharacter found!" true true "(R=1.000000,G=0.052997,B=0.000000,A=1.000000)" _textduration)
      (Math|Integer|IncrementInt (Variables|Default|GetErrorCount)))))

(event Custom|Check%20for%20End%20Level%20Switch
  (bind _textduration (Variables|Default|GetTextDuration))
  ;[1 1 1] Level Checks
  (bind _outactors (Actor|GetAllActorsOfClass "/Game/Blueprints/LevelCreation/EndLevelSwitch.EndLevelSwitch_C"))
  (if (Utilities|Array|IsValidIndex _outactors)
    (Development|PrintString (Utilities|String|Append (Utilities|String|ToString(Integer) (Utilities|Array|Length _outactors)) " End Level Switch found") true true "(R=0.125343,G=1.000000,B=0.000000,A=1.000000)" _textduration)
    (else
      (Development|PrintString "!WARNING! - No End Level Switch found!" true true "(R=1.000000,G=0.038177,B=0.000000,A=1.000000)" _textduration)
      (Math|Integer|IncrementInt (Variables|Default|GetErrorCount)))))

(event Custom|Update%20Death%20List
  (params (DestroyedActor :type Actor%20Object%20Reference))
  ;[1 1 1] Pass Level Name to Player HUD
  (bind _asenemy (Utilities|Casting|CastToEnemy DestroyedActor))
  (Utilities|Array|AddUnique (Variables|Default|GetEnemyDeathList) (Utilities|Struct|MakeDeathStatStruct _asenemy (Transformation|GetActorLocation DestroyedActor) (Utilities|Array|Get(acopy) (Variables|/Game/CoreFiles/Characters/2DChar.2DChar_C|GetAnimationArray _asenemy) 15) (Class|PaperFlipbook|GetNumFrames (Utilities|Array|Get(acopy) (Variables|/Game/CoreFiles/Characters/2DChar.2DChar_C|GetAnimationArray _asenemy) 15)) (Transformation|GetWorldScale (Variables|/Game/CoreFiles/Characters/2DChar.2DChar_C|GetPaperFlipbook _asenemy)) (Transformation|GetActorRotation _asenemy))))

(event Custom|Count%20Enemies
  (bind _textduration (Variables|Default|GetTextDuration))
  ;[1 1 1] Level Checks
  (bind _outactors (Actor|GetAllActorsOfClass "/Game/CoreFiles/Characters/Enemy/Enemy.Enemy_C"))
  (if (Utilities|Array|IsValidIndex _outactors)
    (Development|PrintString (Utilities|String|Append (Utilities|String|ToString(Integer) (Utilities|Array|Length _outactors)) " Enemies found") true true "(R=0.160779,G=1.000000,B=0.000000,A=1.000000)" _textduration)
    (else
      (Development|PrintString "!WARNING! - No Enemies found!" true true "(R=1.000000,G=0.000000,B=0.018362,A=1.000000)" _textduration)
      (Math|Integer|IncrementInt (Variables|Default|GetErrorCount)))))

(event EventBeginPlay
  ;[1 1 1] Pass Level Name to Player HUD
  (Utilities|FlowControl|Sequence
    (:then_0
      (CallFunction|TurnOffWalls)
      (CallFunction|TurnOffCeilings)
      (CallFunction|TurnonWalls)
      (CallFunction|TurnonCeilings))
    (:then_2
      (Utilities|FlowControl|Delay 1.0)
      (bind _outactors (Actor|GetAllActorsOfClass "/Game/Blueprints/Characters/PlayerCharacter.PlayerCharacter_C"))
      (Default|DisplayLevelName (Variables|/Game/Blueprints/Characters/PlayerCharacter.PlayerCharacter_C|GetMyHud (Utilities|Array|Get(acopy) _outactors)) (Variables|Default|GetLevelName)))))

(fn ConstructionScript)