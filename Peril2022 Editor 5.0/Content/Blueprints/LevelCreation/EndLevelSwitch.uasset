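; EndLevelSwitch is an interactable that ends the level and shows the player the end game screen, passing along NextLevel.
; On interact it freezes the player, makes them invincible, hides the crosshair and HUD, and gives mouse input to the stats screen.
; It also stops every Enemy's movement and clears its target-check timer, then calls StartStats on the first LevelHelper found.
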(event EventInteract
  (params (Player :type Player%20Character%20Object%20Reference))
  (bind _returnvalue (Game|GetPlayerController 0))
  ;[1 1 1] On Used
  (Default|ShowEndGameScreen Player (Variables|Default|GetNextLevel))
  (Pawn|Components|CharacterMovement|SetMovementMode (Variables|/Script/Engine.Character|GetCharacterMovement Player) "MOVE_None" 0)
  (Default|ToggleCrosshair Player false)
  (Widget|RemovefromParent (Variables|/Game/Blueprints/Characters/PlayerCharacter.PlayerCharacter_C|GetMyHud Player))
  (Variables|/Script/Engine.PlayerController|SetbShowMouseCursor _returnvalue true)
  (Input|SetInputModeUIOnly _returnvalue (Variables|/Game/Blueprints/Characters/PlayerCharacter.PlayerCharacter_C|GetMyStatsScreen Player) "DoNotLock")
  (Variables|/Game/Blueprints/Characters/PlayerCharacter.PlayerCharacter_C|SetInvincible Player true)
  (bind _outactors (Actor|GetAllActorsOfClass "/Game/CoreFiles/Characters/Enemy/Enemy.Enemy_C"))
  (for _array_element _outactors
    (Pawn|Components|CharacterMovement|SetMovementMode (Variables|/Script/Engine.Character|GetCharacterMovement _array_element) "MOVE_None" 0)
    (if (Class|KismetSystemLibrary|TimerExistsHandle (Variables|/Game/CoreFiles/Characters/Enemy/Enemy.Enemy_C|GetTargetCheckTimer _array_element))
      (Utilities|Time|ClearandInvalidateTimerbyHandle (Variables|/Game/CoreFiles/Characters/Enemy/Enemy.Enemy_C|GetTargetCheckTimer _array_element))))
  (Utilities|FlowControl|Sequence
    (:then_0
      (bind _outactors_2 (Actor|GetAllActorsOfClass "/Game/Blueprints/LevelCreation/LevelHelper.LevelHelper_C"))
      (Default|StartStats (Utilities|Array|Get(acopy) _outactors_2)))))

(fn ConstructionScript)