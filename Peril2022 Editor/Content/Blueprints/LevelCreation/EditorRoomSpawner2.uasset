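; Editor room builder whose construction script lays out a RoomWidth by RoomDepth grid of EditorFloorCube child actors around itself, passing them RoomHeight.
; Wall events trace four directions, ignoring Doors, and stack EditorWall child actors up to RoomHeight on unblocked sides of its own center tile, or clear them.
; Ceiling events add or remove a single EditorWall above that tile.
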(event Custom|Create%20Ceiling
  ;[1 1 1] Create and Destroy Ceiling
  (Utilities|IsValid (Variables|Default|GetMyCeiling)
    (:Is%20Not%20Valid
      (bind _returnvalue (AddComponent|AddChildActorComponent false (Math|Transform|MakeTransform (Math|Vector|MakeVector 0.0 0.0 (* (Variables|Default|GetFloorSize) (Math|Conversions|ToFloat(Integer) (+ (Variables|Default|GetRoomHeight) 1)))) "0, 0, 0" "1,1,1")))
      (ChildActorComponent|SetChildActorClass _returnvalue "/Game/Blueprints/LevelCreation/EditorWall.EditorWall_C")
      (Variables|Default|SetMyCeiling _returnvalue))))

(event Custom|Destroy%20Ceiling
  ;[1 1 1] Create and Destroy Ceiling
  (Utilities|IsValid (Variables|Default|GetMyCeiling)
    (:Is%20Valid
      (Components|DestroyComponent (Variables|Default|GetMyCeiling))
      (Variables|Default|SetMyCeiling 0))))

(event Custom|DestroyWalls
  ;[1 1 1] Destroy Walls
  (for _array_element (Variables|Default|GetMyWalls)
    (Components|DestroyComponent _array_element))
  (Utilities|Array|Clear (Variables|Default|GetMyWalls)))

(event Custom|CreateWalls
  (bind _returnvalue (Transformation|GetActorLocation))
  (bind _returnvalue_2 (Transformation|GetActorLocation))
  (bind _floorsize (Variables|Default|GetFloorSize))
  (bind _returnvalue_3 (* _floorsize -1.0))
  ;[1 1 1] Create Walls
  (bind _outactors (Actor|GetAllActorsOfClass "/Game/Blueprints/LevelCreation/Door.Door_C"))
  (Variables|Default|SetDirection "NewEnumerator0")
  (for _index (range 0 3)
    (bind (_outhit _returnvalue_4) (Collision|LineTraceForObjects _returnvalue_2 (+ _returnvalue_2 (Utilities|Select :Index (Variables|Default|GetDirection) :NewEnumerator0 "200.000000, 0,0.000000" :NewEnumerator1 "-200.000000, 0,0.000000" :NewEnumerator2 "0,-200.000000,0.000000" :NewEnumerator3 "0,200.000000,0.000000")) (Utilities|Array|MakeArray "ObjectTypeQuery1") false _outactors "None"))
    (if _returnvalue_4
      _
      (else
        (for _index_2 (range 0 (Variables|Default|GetRoomHeight))
          (bind _returnvalue_5 (Collision|LineTraceForObjects _returnvalue (+ _returnvalue (+ (Utilities|Select :Index (Variables|Default|GetDirection) :NewEnumerator0 "200.000000, 0,0.000000" :NewEnumerator1 "-200.000000,0.000000,0.000000" :NewEnumerator2 "0.000000,-200.000000,0.000000" :NewEnumerator3 "0.000000,200.000000,0.000000") (Math|Vector|MakeVector 0.0 0.0 (+ (* _index_2 (Variables|Default|GetWallSize)) 2.0)))) (Utilities|Array|MakeArray "ObjectTypeQuery1") false _outactors "None"))
          (if (not _returnvalue_5)
            (bind _returnvalue_6 (AddComponent|AddChildActorComponent false (Math|Transform|MakeTransform (Utilities|Select :Index (Variables|Default|GetDirection) :NewEnumerator0 (Math|Vector|MakeVector _floorsize 0.0 (* _index_2 (Variables|Default|GetWallSize))) :NewEnumerator1 (Math|Vector|MakeVector _returnvalue_3 0.0 (* _index_2 (Variables|Default|GetWallSize))) :NewEnumerator2 (Math|Vector|MakeVector 0.0 _returnvalue_3 (* _index_2 (Variables|Default|GetWallSize))) :NewEnumerator3 (Math|Vector|MakeVector 0.0 _floorsize (* _index_2 (Variables|Default|GetWallSize)))) "0, 0, 0" "1,1,1")))
            (ChildActorComponent|SetChildActorClass _returnvalue_6 "/Game/Blueprints/LevelCreation/EditorWall.EditorWall_C")
            (Utilities|Array|Add (Variables|Default|GetMyWalls) _returnvalue_6)))))
    (Variables|Default|SetDirection (Utilities|Enum|ByteToEnumFloorDirection (+ (Variables|Default|GetDirection) 1)))))

(fn ConstructionScript
  (bind _roomwidth (Variables|Default|GetRoomWidth))
  (bind _floorsize (Variables|Default|GetFloorSize))
  (bind _roomdepth (Variables|Default|GetRoomDepth))
  (bind _returnvalue (/ _roomdepth 2))
  (bind _returnvalue_2 (/ _roomwidth 2))
  (Transformation|SetActorRotation "0, 0, 0")
  (for _index (range (* _returnvalue -1) (- _returnvalue (Utilities|Select :Index (Math|Integer|%(Integer) _roomdepth 2) :Option%200 1 :Option%201 0)))
    (for _index_2 (range (* _returnvalue_2 -1) (- _returnvalue_2 (Utilities|Select :Index (Math|Integer|%(Integer) _roomwidth 2) :Option%200 1 :Option%201 0)))
      (if (or (!= _index_2 0) (!= _index 0))
        (bind _returnvalue_3 (AddComponent|AddChildActorComponent false (Math|Transform|MakeTransform (Math|Vector|MakeVector (* (Math|Conversions|ToFloat(Integer) _index_2) _floorsize) (* _index _floorsize) 0.0) "0, 0, 0" "1,1,1")))
        (ChildActorComponent|SetChildActorClass _returnvalue_3 "/Game/Blueprints/LevelCreation/EditorFloorCube.EditorFloorCube_C")))
    (for _array_element (Actor|GetAllChildActors true)
      (Variables|/Script/Engine.Actor|SetTags _array_element (Utilities|Array|MakeArray "RoomFloor"))
      (bind _aseditor_floor_cube (Utilities|Casting|CastToEditorFloorCube _array_element))
      (Variables|/Game/Blueprints/LevelCreation/EditorFloorCube.EditorFloorCube_C|SetRoomHeight _aseditor_floor_cube (Variables|Default|GetRoomHeight)))))