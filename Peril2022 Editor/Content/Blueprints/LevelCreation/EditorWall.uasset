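; Editor wall actor for level creation that varies the look of its static mesh through material slots 2 to 5.
; The Construction Script calls RandomiseMaterial, which gives each slot a 40% chance of a random wall material variant.
; A separate ChangeTheme event sets those slots by Space Base, Castle or Facility theme.
; The Construction Script's lookup of LevelHelper's theme is disconnected, so it never applies the theme.
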(event Custom|RandomiseMaterial
  (for _index (range 2 5)
    (if (<= (Math|Random|RandomFloat) 0.4)
      (Rendering|Material|SetMaterial (Variables|Default|GetStaticMesh) _index (Utilities|Select :Index (Math|Random|RandomInteger 4) :Option%200 "/Game/CoreFiles/Graphics/World/Walls/wall02_Mat_Inst.wall02_Mat_Inst" :Option%201 "/Game/CoreFiles/Graphics/World/Walls/wall03_Mat_Inst.wall03_Mat_Inst" :Option%202 "/Game/CoreFiles/Graphics/World/Walls/wall05_Mat_Inst.wall05_Mat_Inst" :Option%203 "/Game/CoreFiles/Graphics/World/Walls/Wall06_Mat_Inst.Wall06_Mat_Inst" :Option%204 "/Game/CoreFiles/Graphics/World/Walls/wall01_Mat_Inst.wall01_Mat_Inst")))))

(event Custom|ChangeTheme
  (params (Theme :type ThemeEnum%20Enum :default "NewEnumerator0"))
  (for _index (range 2 5)
    (Rendering|Material|SetMaterial (Variables|Default|GetStaticMesh) _index (Utilities|Select :Index Theme :NewEnumerator0 "/Game/CoreFiles/Graphics/World/Walls/wall01_Mat_Inst.wall01_Mat_Inst" :NewEnumerator1 "/Game/CoreFiles/Graphics/World/CastleWall.CastleWall" :NewEnumerator2 "/Game/CoreFiles/Graphics/World/Walls/wall01_Mat_Inst.wall01_Mat_Inst"))))

(event EventBeginPlay)

(event Collision|EventActorBeginOverlap
  (params (OtherActor :type Actor%20Object%20Reference)))

(event EventTick
  (params (DeltaSeconds :type Float%20%28single-precision%29)))

(fn ConstructionScript
  (CallFunction|RandomiseMaterial))