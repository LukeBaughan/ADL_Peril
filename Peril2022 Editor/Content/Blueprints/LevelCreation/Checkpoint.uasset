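; Checkpoint pickup that sets the player's respawn transform to its own location and rotation when a PlayerCharacter overlaps its box.
; On that overlap it shows a "Checkpoint!" HUD notification, then destroys itself.
; A timeline repeatedly animates the sprite along the vertical axis, restarting itself on finish.
; While recently rendered, Tick turns the Arrow component toward the player camera.
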(event OnComponentBeginOverlap(Box)
  (params (OverlappedComponent :type Primitive%20Component%20Object%20Reference) (OtherActor :type Actor%20Object%20Reference) (OtherComp :type Primitive%20Component%20Object%20Reference) (OtherBodyIndex :type Integer) (bFromSweep :type Boolean) (SweepResult :type Hit%20Result%20Structure%20%28by%20ref%29))
  (bind _asplayer_character (Utilities|Casting|CastToPlayerCharacter OtherActor))
  (Utilities|FlowControl|DoOnce false
    (:Completed
      (Default|DisplayNotification (Variables|/Game/Blueprints/Characters/PlayerCharacter.PlayerCharacter_C|GetMyHud _asplayer_character) "Checkpoint!" false)
      (Variables|/Game/Blueprints/Characters/PlayerCharacter.PlayerCharacter_C|SetSpawnTransform _asplayer_character (Math|Transform|MakeTransform (Transformation|GetActorLocation) (Transformation|GetActorRotation) "1,1,1"))
      (Actor|DestroyActor))))

(event Custom|MoveSprite
  (Components|Timeline|SetPlayRate (Variables|Default|GetMoveSpriteTL) 0.3)
  (Variables|Default|SetStartLoc (Transformation|GetWorldLocation (Variables|Default|GetPaperSprite)))
  (bind _newtrack_0 (Timeline|MoveSpriteTL PlayFromStart)
    (:Update
      (Transformation|SetWorldLocation (Variables|Default|GetPaperSprite) (Math|Vector|Lerp(Vector) (Variables|Default|GetStartLoc) (Math|Vector|MakeVector (.X (Math|Vector|BreakVector (Variables|Default|GetStartLoc))) (.Y (Math|Vector|BreakVector (Variables|Default|GetStartLoc))) (+ (.Z (Math|Vector|BreakVector (Variables|Default|GetStartLoc))) 1e+02)) _newtrack_0) false false))
    (:Finished
      (CallFunction|MoveSprite))))

(event EventBeginPlay
  (CallFunction|MoveSprite))

(event EventTick
  (params (DeltaSeconds :type Float%20%28single-precision%29))
  (if (Class|Actor|WasRecentlyRendered 0.2)
    (Transformation|SetWorldRotation (Variables|Default|GetArrow) (Math|Rotator|FindLookatRotation (Transformation|GetActorLocation) (Camera|GetCameraLocation (Game|GetPlayerCameraManager 0))) false false)))

(fn ConstructionScript)