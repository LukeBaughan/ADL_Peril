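; Level door that slides up on a timeline, with a lock type of key, switch, enemy portal or boss.
; The construction script tints both faces by lock type and sets optional boss-skull sprites.
; Interact toggles the door or shows a lock notification, TriggerResponse toggles it without a lock check, and enemies auto-open unlocked doors.
; Opening can shake the camera, and a closed door reopens if pawns overlap its trigger.
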(event OnComponentBeginOverlap(TriggerOpen)
  (params (OverlappedComponent :type Primitive%20Component%20Object%20Reference) (OtherActor :type Actor%20Object%20Reference) (OtherComp :type Primitive%20Component%20Object%20Reference) (OtherBodyIndex :type Integer) (bFromSweep :type Boolean) (SweepResult :type Hit%20Result%20Structure%20%28by%20ref%29))
  (bind _dooropen (Variables|Default|GetDoorOpen))
  ;[1 1 1] Collision Events
  (Utilities|Casting|CastToEnemy OtherActor)
  (if (Utilities|Enum|Equal(Enum) (Variables|Default|GetRequired) "NewEnumerator0")
    (if (not (Audio|Components|Audio|IsPlaying _dooropen))
      (if (Class|TimelineComponent|IsReversing _dooropen)
        (CallFunction|DoorOpen :!label _label)
        (elif (== (Components|Timeline|GetPlaybackPosition _dooropen) 0.0)
          (goto _label))))))

(event OnComponentEndOverlap(TriggerOpen)
  (params (OverlappedComponent :type Primitive%20Component%20Object%20Reference) (OtherActor :type Actor%20Object%20Reference) (OtherComp :type Primitive%20Component%20Object%20Reference) (OtherBodyIndex :type Integer))
  ;[1 1 1] Collision Events
  (Utilities|Casting|CastToEnemy OtherActor))

(event Custom|Door%20Open
  ;[1 1 1] Open / Close Animation
  (if (Variables|Default|GetRumble?)
    (CameraShakes|StartCameraShake (Game|GetPlayerCameraManager 0) "/Game/CoreFiles/Characters/MediumCameraShake.MediumCameraShake_C" 0.2 "CameraLocal" "0, 0, 0"))
  (Components|Timeline|SetPlayRate (Variables|Default|GetDoorOpen) (Variables|Default|GetSpeed))
  (Variables|Default|SetStartLoc (Variables|/Script/Engine.SceneComponent|GetRelativeLocation (Variables|Default|GetDoor)))
  (bind (_direction _newtrack_0) (Timeline|DoorOpen Play)
    (:Update
      (Transformation|SetRelativeLocation (Variables|Default|GetDoor) (Math|Vector|Lerp(Vector) (Variables|Default|GetStartLoc) (Math|Vector|MakeVector (.X (Math|Vector|BreakVector (Variables|Default|GetStartLoc))) (.Y (Math|Vector|BreakVector (Variables|Default|GetStartLoc))) 2.5e+02) _newtrack_0) false false))
    (:Finished
      (switch Utilities|FlowControl|Switch|SwitchonETimelineDirection _direction
        (:Forward
          (Variables|Default|SetOpen? true))
        (:Backward
          (Variables|Default|SetOpen? false)
          (if (Utilities|Array|IsValidIndex (Collision|GetOverlappingActors (Variables|Default|GetTriggerOpen) "/Script/Engine.Pawn" :!class /Script/Engine.PrimitiveComponent))
            (CallFunction|DoorOpen)))))))

(event Custom|Door%20Close
  (bind _startloc (Variables|Default|GetStartLoc))
  (bind (_x _y) (Math|Vector|BreakVector _startloc))
  ;[1 1 1] Open / Close Animation
  (bind (_direction _newtrack_0) (Timeline|DoorOpen Reverse)
    (:Update
      (Transformation|SetRelativeLocation (Variables|Default|GetDoor) (Math|Vector|Lerp(Vector) _startloc (Math|Vector|MakeVector _x _y 2.5e+02) _newtrack_0) false false))
    (:Finished
      (switch Utilities|FlowControl|Switch|SwitchonETimelineDirection _direction
        (:Forward
          (Variables|Default|SetOpen? true))
        (:Backward
          (Variables|Default|SetOpen? false)
          (if (Utilities|Array|IsValidIndex (Collision|GetOverlappingActors (Variables|Default|GetTriggerOpen) "/Script/Engine.Pawn" :!class /Script/Engine.PrimitiveComponent))
            (CallFunction|DoorOpen)))))))

(event Custom|Update%20Light%20Colour
  ;[1 1 1] Change Light
  (Rendering|Material|SetVectorParameterValueonMaterials (Variables|Default|GetDoor%20Front) "DoorColour" (Math|Conversions|ToVector(LinearColor) (Utilities|Select :Index (Variables|Default|GetRequired) :NewEnumerator0 "(R=1.000000,G=1.000000,B=1.000000,A=1.000000)" :NewEnumerator1 "(R=1.000000,G=0.000000,B=0.000000,A=1.000000)" :NewEnumerator2 "(R=0.000000,G=0.056797,B=1.000000,A=1.000000)" :NewEnumerator3 "(R=0.000000,G=0.385417,B=0.049622,A=1.000000)" :NewEnumerator4 "(R=1.000000,G=0.970675,B=0.000000,A=1.000000)" :NewEnumerator5 "(R=1.000000,G=0.000000,B=0.850150,A=1.000000)" :NewEnumerator6 "(R=1.000000,G=0.000000,B=0.744212,A=1.000000)"))))

(event Custom|Update%20Deco
  (bind _deco (Variables|Default|GetDeco))
  (bind _returnvalue (Utilities|Select :Index _deco :NewEnumerator0 0 :NewEnumerator1 "/Game/CoreFiles/Graphics/World/bossskull_Sprite.bossskull_Sprite"))
  ;[1 1 1] Update Deco
  (Rendering|Components|Sprite|SetSprite (Variables|Default|GetDeco%20Front) _returnvalue)
  (Rendering|Components|Sprite|SetSprite (Variables|Default|GetDeco%20Back) _returnvalue))

(event EventInteract
  (params (Player :type Player%20Character%20Object%20Reference))
  (bind _required (Variables|Default|GetRequired))
  (bind _dooropen (Variables|Default|GetDoorOpen))
  ;[1 1 1] Collision Events
  (if (Utilities|Enum|Equal(Enum) _required "NewEnumerator0")
    (if true :!label _label
      (if (Audio|Components|Audio|IsPlaying _dooropen)
        (CallFunction|DoorClose)
        (elif (Class|TimelineComponent|IsReversing _dooropen)
          (CallFunction|DoorOpen :!label _label_2)
          (elif (== (Components|Timeline|GetPlaybackPosition _dooropen) 0.0)
            (goto _label_2)
            (else
              (CallFunction|DoorClose)))))
      (else
        (goto _label_2)))
    (elif (Math|Boolean|ORBoolean (and (Utilities|Enum|Equal(Enum) _required "NewEnumerator1") (Utilities|CheckKey Player "NewEnumerator0")) (and (Utilities|Enum|Equal(Enum) _required "NewEnumerator2") (Utilities|CheckKey Player "NewEnumerator1")) (and (Utilities|Enum|Equal(Enum) _required "NewEnumerator3") (Utilities|CheckKey Player "NewEnumerator2")))
      (goto _label)
      (elif (not (Variables|Default|GetOpen?))
        (Default|DisplayNotification (Variables|/Game/Blueprints/Characters/PlayerCharacter.PlayerCharacter_C|GetMyHud Player) (Utilities|Select :Index _required :NewEnumerator0 "" :NewEnumerator1 "Red Key required" :NewEnumerator2 "Blue Key required" :NewEnumerator3 "Green Key required" :NewEnumerator4 "Door is operated  by a switch" :NewEnumerator5 "Door is locked by a nearbye Portal" :NewEnumerator6 "Door is locked by a powerful enemy") false)))))

(event EventTriggerResponse
  (bind _dooropen (Variables|Default|GetDoorOpen))
  ;[1 1 1] Collision Events
  (if true
    (if (Audio|Components|Audio|IsPlaying _dooropen)
      (CallFunction|DoorClose)
      (elif (Class|TimelineComponent|IsReversing _dooropen)
        (CallFunction|DoorOpen :!label _label)
        (elif (== (Components|Timeline|GetPlaybackPosition _dooropen) 0.0)
          (goto _label)
          (else
            (CallFunction|DoorClose)))))
    (else
      (goto _label))))

(event EventBeginPlay
  (Variables|Default|SetDefaultRequired (Variables|Default|GetRequired)))

(fn ConstructionScript
  (CallFunction|UpdateLightColour)
  (CallFunction|UpdateDeco))